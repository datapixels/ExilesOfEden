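; Enemy gameplay ability that performs a ranged attack by firing a projectile at the avatar's combat target.
; On activation it gets the target and a random attack montage from the avatar through messages, turns the avatar toward the target, and plays the montage.
; The montage's gameplay event tag times the projectile spawn at the target's location at that moment.
; The ability ends shortly after firing, or when the montage completes or is interrupted.
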(event Ability|EventActivateAbility
  (bind _returnvalue (Ability|GetAvatarActorfromActorInfo))
  (bind _returnvalue_2 (Class|TargetInterface|GetCombatTarget(Message) (Ability|GetAvatarActorfromActorInfo)))
  (Variables|Default|SetCombatTarget _returnvalue_2)
  (Class|CombatInterface|UpdateFacingTarget(Message) _returnvalue (Transformation|GetActorLocation _returnvalue_2))
  (bind _returnvalue_3 (Class|CombatInterface|GetRandomAttackMontage(Message) _returnvalue))
  (|PlayMontageandWaitProxy "None" (.Montage (Utilities|Struct|BreakTaggedMontage _returnvalue_3)) 1.0 "None" false 1.0 0.0 false
    (:then
      (Ability|Tasks|WaitGameplayEvent (.MontageTag (Utilities|Struct|BreakTaggedMontage _returnvalue_3)) 0
        (:EventReceived
          (Class|CombatInterface|GetCombatSocketsLocation(Message) (Ability|GetAvatarActorfromActorInfo) (.MontageTag (Utilities|Struct|BreakTaggedMontage _returnvalue_3)))
          (Class|AuraProjectileSpell|SpawnProjectile (Transformation|GetActorLocation (Variables|Default|GetCombatTarget)))
          (Utilities|FlowControl|Delay 0.2)
          (Ability|EndAbility))))
    (:OnCompleted
      (Ability|EndAbility :!label _label))
    (:OnInterrupted
      (goto _label))
    (:OnCancelled
      (goto _label))))

(event Ability|EventOnEndAbility
  (params (bWasCancelled :type Boolean)))